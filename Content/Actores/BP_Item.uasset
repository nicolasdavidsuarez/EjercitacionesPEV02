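; BP_Item is an item Blueprint that reports its values through on-screen debug text.
; MostrarDistancia chains PrintString and Delay nodes to show a "la distancia es" message with growing dots, then prints Distancia.
; MostrarEscudo immediately prints Salud, the health variable, despite its shield name.
; Both are custom events with no caller in this graph; BeginPlay and the construction script are empty.
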(event EventBeginPlay)

(event Collision|EventActorBeginOverlap
  (params (OtherActor :type Actor%20Object%20Reference)))

(event EventTick
  (params (DeltaSeconds :type Float%20%28single-precision%29)))

(event EventMostrarEscudo
  (Development|PrintString (Utilities|String|ToString(Integer) (Variables|Default|Getsalud))))

(event EventMostrarDistancia
  (Development|PrintString "la distancia es" true true "(R=0.000000,G=0.660000,B=1.000000,A=1.000000)" 1.0)
  (Utilities|FlowControl|Delay 1.0)
  (Development|PrintString "la distancia es." true true "(R=0.000000,G=0.660000,B=1.000000,A=1.000000)" 1.0)
  (Utilities|FlowControl|Delay 1.0)
  (Development|PrintString "la distancia es.." true true "(R=0.000000,G=0.660000,B=1.000000,A=1.000000)" 1.0)
  (Utilities|FlowControl|Delay 1.0)
  (Development|PrintString "la distancia es..." true true "(R=0.000000,G=0.660000,B=1.000000,A=1.000000)" 1.5)
  (Utilities|FlowControl|Delay 1.5)
  (Development|PrintString (Utilities|String|ToString(Integer) (Variables|Default|Getdistancia))))

(fn ConstructionScript)